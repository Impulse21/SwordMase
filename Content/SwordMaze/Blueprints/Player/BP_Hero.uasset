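; BP_Hero is the player hero Blueprint in SwordMaze, with an empty construction script and only disabled placeholder events.
; Its one piece of logic, GetCharacterInfo, packs animation state flags for blocking, attack intent, sprint intent and magic use from player input and state variables.
; Blocking is suppressed during the attack-blocked montage, and sprint intent requires being free to animate and not blocking.
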(event EventBeginPlay)

(event Collision|EventActorBeginOverlap
  (params (OtherActor :type Actor%20Object%20Reference)))

(event EventTick
  (params (DeltaSeconds :type Float%20%28single-precision%29)))

(fn ConstructionScript)

(fn GetCharacterInfo
  (bind _playerinput (Variables|Default|GetPlayerInput))
  (bind _returnvalue (Animation|GetCurrentMontage :!class /Script/Engine.Character))
  (return (Utilities|Struct|MakeCharacterAnimationInfo (and (Variables|Default|GetBlocking) (!= _returnvalue "/Game/KnightsOfCouch/Animations/Player/AM_Player_Attack_Blocked.AM_Player_Attack_Blocked")) (.attackpressed _playerinput) (Math|Boolean|ANDBoolean (.holdingsprint _playerinput) (Variables|Default|GetFreeToAnimate) (not (Variables|Default|GetBlocking))) (Variables|Default|GetIsUsingMagic))))