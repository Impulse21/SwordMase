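; BP_DmgArea is a world damage volume that hurts characters standing inside it over time.
; Begin and end overlap events add or remove BaseCharacter actors from a tracked list.
; A looping timer started on BeginPlay fires at a configurable rate and applies environmental damage to every listed actor, with debug prints along the way.
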(event Custom|DamageOverTime
  ;[1 1 1] Damage Over Time
  (for _array_element (Variables|Default|GetActorsToDmg)
    (Game|Damage|ApplyDamage _array_element (Variables|Default|GetDamage) 0 self "/Engine/EngineDamageTypes/DmgTypeBP_Environmental.DmgTypeBP_Environmental_C")
    (Development|PrintString "Appling Damage" true true "(R=1.000000,G=0.133002,B=0.000000,A=1.000000)")))

(event EventBeginPlay
  ;[1 1 1] Damage Over Time
  (Utilities|Time|SetTimerbyEvent (delegate Custom|DamageOverTime) (Variables|Default|GetDamageRate) true))

(event Collision|EventActorBeginOverlap
  (params (OtherActor :type Actor%20Object%20Reference))
  ;[1 1 1] Adding and removing items from the list
  (bind _asbase_character (Utilities|Casting|CastToBaseCharacter OtherActor))
  (Utilities|Array|AddUnique (Variables|Default|GetActorsToDmg) _asbase_character)
  (Development|PrintString "Added Item from damage list"))

(event Collision|EventActorEndOverlap
  (params (OtherActor :type Actor%20Object%20Reference))
  ;[1 1 1] Adding and removing items from the list
  (bind _asbase_character (Utilities|Casting|CastToBaseCharacter OtherActor))
  (Utilities|Array|RemoveItem (Variables|Default|GetActorsToDmg) _asbase_character)
  (Development|PrintString "Removed Item from damage List" true true "(R=1.000000,G=0.067083,B=0.319111,A=1.000000)"))

(fn ConstructionScript)